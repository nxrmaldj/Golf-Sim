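; BP_MovingBall is an actor that travels in a straight line along the world X axis once launched.
; A LaunchShot event sets a moving flag, and Tick then applies a frame-rate-independent offset scaled by Speed.
; The movement is swept, so a blocking hit clears the flag and stops the ball.
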(event Custom|LaunchShot
  ;[0.15 0.15 0.15 0.5] Press space to launchball/ Level Blueprint
  (Variables|Components|SetbIsMoving true))

(event EventBeginPlay)

(event Collision|EventActorBeginOverlap
  (params (OtherActor :type Actor%20Object%20Reference)))

(event EventTick
  (params (DeltaSeconds :type Float%20%28single-precision%29))
  ;[0.15 0.15 0.15 0.5] Controls the Speed of the ball
  (if (Variables|Components|GetbIsMoving)
    (bind _sweephitresult (Transformation|AddActorWorldOffset (Math|Vector|MakeVector (* DeltaSeconds (Variables|Components|GetSpeed)) 0.0 0.0) true))
    (if (.bBlockingHit (Collision|BreakHitResult _sweephitresult))
      (Variables|Components|SetbIsMoving false))))

(fn ConstructionScript)